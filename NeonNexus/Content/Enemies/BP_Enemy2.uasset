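; BP_Enemy2 is an enemy that follows the player when the player is between an inner and outer distance band.
; Each Tick, after a tiny Delay, it checks that range; until FirstMove clears, it plays a PaperZD activation animation override and waits several seconds.
; It then adds scaled movement input toward the player and flips its yaw between two facings based on which side the player is on along Y.
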(event `self.ReceiveTick`
  (params (DeltaSeconds :type "Float (single-precision)"))
  (bind _returnvalue (`self.K2_GetActorLocation`))
  (bind (_returnvalue_x _returnvalue_y) (`KismetMathLibrary.BreakVector` (`self.K2_GetActorLocation`)))
  (bind _returnvalue_2 (`self.K2_GetActorLocation` (`GameplayStatics.GetPlayerPawn` 0)))
  (bind (_returnvalue_x_2 _returnvalue_y_2) (`KismetMathLibrary.BreakVector` (`self.K2_GetActorLocation` (`GameplayStatics.GetPlayerPawn` 0))))
  (bind _returnvalue_3 (`KismetMathLibrary.VSize` (- _returnvalue _returnvalue_2)))
  ;[1 1 1] Moving logic for enemy
  (`KismetSystemLibrary.Delay` 0.001)
  (if (and (< _returnvalue_3 500.0) (> _returnvalue_3 300.0))
    (if (`self.FirstMove`)
      (`PaperZDPlaySlotOverrideAction.PlayAnimationOverrideWithCallbacks` (`self.GetAnimInstance`) "/Game/Enemies/AnimSequences/AS_Enemy2_Active.AS_Enemy2_Active" "Enemy2"
        (:`then`
          (`KismetSystemLibrary.Delay` 5.0)
          (set `self.FirstMove` false))))
    (`self.AddMovementInput` (- _returnvalue_2 _returnvalue) 0.002)
    (`self.K2_SetActorRotation` (`KismetMathLibrary.MakeRotator` 0.0 0.0 (`KismetMathLibrary.SelectFloat` 180.0 0.0 (> (- _returnvalue_y _returnvalue_y_2) 0.0))))))

(fn `UserConstructionScript`)