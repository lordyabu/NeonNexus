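; BP_Enemy2New is an enemy that approaches the player pawn and attacks at close range, with all logic driven from Tick by distance checks.
; At mid range it plays a one-time activation animation, then moves toward the player, flipping yaw to face along Y.
; Up close it plays a shoot animation override, pausing Tick until completion, then calls ShootProjectile, which is empty here.
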(event `self.ReceiveTick`
  (params (DeltaSeconds :type "Float (single-precision)"))
  (bind _returnvalue (`self.GetAnimInstance`))
  (bind _returnvalue_2 (`self.K2_GetActorLocation`))
  (bind (_returnvalue_x _returnvalue_y) (`KismetMathLibrary.BreakVector` (`self.K2_GetActorLocation`)))
  (bind _returnvalue_3 (`self.K2_GetActorLocation` (`GameplayStatics.GetPlayerPawn` 0)))
  (bind (_returnvalue_x_2 _returnvalue_y_2) (`KismetMathLibrary.BreakVector` (`self.K2_GetActorLocation` (`GameplayStatics.GetPlayerPawn` 0))))
  (bind _returnvalue_4 (`KismetMathLibrary.VSize` (- _returnvalue_2 _returnvalue_3)))
  ;[1 1 1] Moving logic for enemy
  (`KismetSystemLibrary.Delay` 0.001)
  (if (and (< _returnvalue_4 750.0) (> _returnvalue_4 300.0))
    (if (`self.FirstMove`)
      (`self.SetActorTickEnabled` false)
      (`PaperZDPlaySlotOverrideAction.PlayAnimationOverrideWithCallbacks` _returnvalue "/Game/Enemies/AnimSequences/AS_Enemy2_Active.AS_Enemy2_Active" "Enemy2"
        (:`OnCompleted`
          (`self.SetActorTickEnabled` true)
          (set `self.FirstMove` false))))
    (`self.AddMovementInput` (- _returnvalue_3 _returnvalue_2) 0.002)
    (`self.K2_SetActorRotation` (`KismetMathLibrary.MakeRotator` 0.0 0.0 (`KismetMathLibrary.SelectFloat` 180.0 0.0 (> (- _returnvalue_y _returnvalue_y_2) 0.0))))
    (elif (<= _returnvalue_4 310.0)
      (`self.SetActorTickEnabled` false)
      (`PaperZDPlaySlotOverrideAction.PlayAnimationOverrideWithCallbacks` _returnvalue "/Game/Enemies/AnimSequences/AS_Enemy2-shoot.AS_Enemy2-shoot" "Enemy2"
        (:`OnCompleted`
          (`self.SetActorTickEnabled` true)
          (`self.Shoot Projectile`))))))

(event `Shoot Projectile`)

(fn `UserConstructionScript`)