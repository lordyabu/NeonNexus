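; BP_LevelComplete is a level-end trigger that moves the player to the next level.
; When a Knight overlaps its Box, it shows the WBP_Complete widget for a one-second delay, then removes it.
; A hard-coded switch on the current level name opens the following tile level by name.
; Any level name outside the switch shows the Game_Complete widget instead of loading a level.
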(event `self.Box.OnComponentBeginOverlap`
  (params (OverlappedComponent :type "PrimitiveComponent Object Reference") (OtherActor :type "Actor Object Reference") (OtherComp :type "PrimitiveComponent Object Reference") (OtherBodyIndex :type Integer) (bFromSweep :type Boolean) (SweepResult :type "HitResult Structure (by ref)"))
  (cast `/Game/SideScrollerBP/Blueprints/Knight` OtherActor)
  (bind _returnvalue (`|CreateWidget` "/Game/Environments/WBP_Complete.WBP_Complete_C"))
  (`UserWidget.AddToViewport` _returnvalue 0)
  (bind _returnvalue_2 (`GameplayStatics.GetCurrentLevelName` true))
  (`KismetSystemLibrary.Delay` 1.0)
  (`Widget.RemoveFromParent` _returnvalue)
  (switch `string` _returnvalue_2
    (:`Default`
      (bind _returnvalue_3 (`|CreateWidget` "/Game/Environments/Game_Complete.Game_Complete_C"))
      (`UserWidget.AddToViewport` _returnvalue_3 0))
    (:`Level0_Tile`
      (bind _output_get (set `self.ToLoad` "Level1_Tile"))
      (`GameplayStatics.OpenLevel` (`KismetStringLibrary.Conv_StringToName` _output_get)))
    (:`Level1_Tile`
      (bind _output_get_2 (set `self.ToLoad` "Level2_Tile"))
      (`GameplayStatics.OpenLevel` (`KismetStringLibrary.Conv_StringToName` _output_get_2)))
    (:`Level2_Tile`
      (bind _output_get_3 (set `self.ToLoad` "Level3_Tile"))
      (`GameplayStatics.OpenLevel` (`KismetStringLibrary.Conv_StringToName` _output_get_3)))))

(fn `UserConstructionScript`)