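; Invincibility pickup actor that grants a Knight temporary invincibility on touch.
; A box overlap hides the actor, saves the Knight's Health and sets it to a huge value while showing the Invincibility widget created at BeginPlay.
; After a short delay it removes the widget, restores the saved Health and destroys itself.
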(event `self.ReceiveBeginPlay`
  (bind _returnvalue (`|CreateWidget` "/Game/Environments/Invincibility/Invincibility_WBP.Invincibility_WBP_C"))
  (set `self.widget` _returnvalue))

(event `self.Box.OnComponentBeginOverlap`
  (params (OverlappedComponent :type "PrimitiveComponent Object Reference") (OtherActor :type "Actor Object Reference") (OtherComp :type "PrimitiveComponent Object Reference") (OtherBodyIndex :type Integer) (bFromSweep :type Boolean) (SweepResult :type "HitResult Structure (by ref)"))
  (bind _asknight (cast `/Game/SideScrollerBP/Blueprints/Knight` OtherActor))
  (`self.SetActorHiddenInGame` true)
  (set `self.SaveHealth` (`/Game/SideScrollerBP/Blueprints/Knight.Health` _asknight))
  (set `/Game/SideScrollerBP/Blueprints/Knight.Health` 1000000.0 _asknight)
  (`UserWidget.AddToViewport` (`self.widget`) 0)
  (`KismetSystemLibrary.Delay` 4.0)
  (`Widget.RemoveFromParent` (`self.widget`))
  (set `/Game/SideScrollerBP/Blueprints/Knight.Health` (`self.SaveHealth`) _asknight)
  (`self.K2_DestroyActor`))

(fn `UserConstructionScript`)